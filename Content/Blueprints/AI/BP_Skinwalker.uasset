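; Skinwalker AI pawn that chases the player once it detects a pawn.
; PawnSensing sets a visibility flag, which nothing here clears, and calls followPlayer to run AI MoveTo on player character 0.
; A debug input shows the Skinwalker's health on screen and at its location on every other press.
; The Damage section holds only this debug display, with no damage handling.
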(event `followPlayer`
  ;[0 0.1282 1] Movement & Player visibility
  (if (`self.playerVis`)
    (`|AIMoveTo` self (0.0 0.0 0.0) (`GameplayStatics.GetPlayerCharacter` 0))))

(event `InputAction|showDebug`
  (params (Key :type "Key Structure"))
  (bind _returnvalue (`KismetStringLibrary.Conv_DoubleToString` (`self.SWHealth`)))
  ;[1 1 1] Damage
  (:`Pressed`
    (`/Engine/EditorBlueprintResources/StandardMacros.FlipFlop`
      (:`A`
        (`KismetSystemLibrary.PrintString` _returnvalue)
        (`KismetSystemLibrary.DrawDebugString` (`self.K2_GetActorLocation`) _returnvalue null (struct :`R` 1.0 :`A` 1.0))))))

(event `self.PawnSensing.OnSeePawn`
  (params (Pawn :type "Pawn Object Reference"))
  ;[0 0.1282 1] Movement & Player visibility
  (set `self.playerVis` true)
  (`self.followPlayer`))

(fn `UserConstructionScript`)